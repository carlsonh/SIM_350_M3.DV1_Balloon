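; Balloon actor that floats upward and can be grabbed and released through a pickup interface.
; While its static mesh simulates physics, Tick applies a randomised impulse within a narrow upward cone each frame, unscaled by delta time, for wobbly lift.
; Pickup turns physics off and attaches to the supplied component, which also stops the lift.
; Drop detaches it and re-enables physics, so it rises again.
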(event EventBeginPlay)

(event Collision|EventActorBeginOverlap
  (params (OtherActor :type Actor%20Object%20Reference)))

(event EventTick
  (params (DeltaSeconds :type Float%20%28single-precision%29))
  (if (Physics|IsSimulatingPhysics (Variables|Default|GetStaticMesh) "None")
    (Physics|AddImpulse (Variables|Default|GetStaticMesh) (* (Math|Random|RandomUnitVectorinConeinDegrees "0, 0,1.000000" 15.0) 5e+02) "None" false)))

(event EventPickup
  (params (AttachTo :type Scene%20Component%20Object%20Reference))
  (Physics|SetSimulatePhysics (Variables|Default|GetStaticMesh) false)
  (Transformation|AttachComponentToComponent AttachTo "None" "KeepWorld" "KeepWorld" "KeepWorld" true))

(event EventDrop
  (Transformation|DetachFromActor "KeepWorld" "KeepWorld" "KeepWorld")
  (Physics|SetSimulatePhysics (Variables|Default|GetStaticMesh) true))

(fn ConstructionScript)