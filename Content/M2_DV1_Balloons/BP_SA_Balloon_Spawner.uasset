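; BP_SA_Balloon_Spawner is a pickup actor that inflates and releases balloons with the left trigger while held.
; Its pickup interface attaches it, toggles cube physics and enables player input only while carried.
; Pressing spawns a zero-scale balloon on the spawn point and opens a gate that lets trigger axis values grow it uniformly.
; Releasing closes the gate, detaches the balloon and turns on its physics.
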(event Input|ActionEvents|InputActionTrigger_L
  (params (Key :type Key%20Structure :default "None"))
  (:Pressed
    (bind _returnvalue (Game|SpawnActorfromClass "/Game/M2_DV1_Balloons/BP_SA_Balloon.BP_SA_Balloon_C" (Transformation|GetWorldTransform (Variables|Default|GetBalloon_Spawn_Point)) "AlwaysSpawn" self 0))
    (Transformation|SetRelativeScale3D (Variables|/Script/Engine.Actor|GetRootComponent _returnvalue) "0, 0, 0")
    (Transformation|AttachComponentToComponent _returnvalue (Variables|Default|GetBalloon_Spawn_Point) "None" "SnapToTarget" "SnapToTarget" "KeepRelative" true))
  (:Released
    (Utilities|FlowControl|Gate true) ; enters at Close
  ))

(event Input|ActionEvents|InputActionTrigger_L
  (params (Key :type Key%20Structure :default "None"))
  (:Pressed
    (Utilities|FlowControl|Gate true) ; enters at Open
  )
  (:Released
    (Transformation|DetachFromActor (stale _returnvalue) "KeepWorld" "KeepWorld" "KeepWorld")
    (Physics|SetSimulatePhysics (Variables|/Game/M2_DV1_Balloons/BP_SA_Balloon.BP_SA_Balloon_C|GetStaticMesh (stale _returnvalue)) true)))

(event Input|AxisEvents|InputAxisTrigger_L_Axis
  (params (AxisValue :type Float%20%28single-precision%29))
  (Utilities|FlowControl|Gate true
    (:Exit
      (Utilities|IsValid (stale Input|ActionEvents|InputActionTrigger_L _returnvalue)
        (:Is%20Valid
          (Transformation|SetRelativeScale3D (Variables|/Script/Engine.Actor|GetRootComponent (stale Input|ActionEvents|InputActionTrigger_L _returnvalue)) (Math|Vector|MakeVector (+ (.Z (Math|Vector|BreakVector (Variables|/Script/Engine.SceneComponent|GetRelativeScale3D (Variables|/Script/Engine.Actor|GetRootComponent (stale Input|ActionEvents|InputActionTrigger_L _returnvalue))))) (/ AxisValue 5e+02)) (+ (.Z (Math|Vector|BreakVector (Variables|/Script/Engine.SceneComponent|GetRelativeScale3D (Variables|/Script/Engine.Actor|GetRootComponent (stale Input|ActionEvents|InputActionTrigger_L _returnvalue))))) (/ AxisValue 5e+02)) (+ (.Z (Math|Vector|BreakVector (Variables|/Script/Engine.SceneComponent|GetRelativeScale3D (Variables|/Script/Engine.Actor|GetRootComponent (stale Input|ActionEvents|InputActionTrigger_L _returnvalue))))) (/ AxisValue 5e+02)))))))))

(event EventPickup
  (params (AttachTo :type Scene%20Component%20Object%20Reference))
  (Physics|SetSimulatePhysics (Variables|Default|GetCube) false)
  (Transformation|AttachComponentToComponent AttachTo "None" "KeepWorld" "KeepWorld" "KeepWorld" true)
  (Input|EnableInput (Game|GetPlayerController 0)))

(event EventDrop
  (Transformation|DetachFromActor "KeepWorld" "KeepWorld" "KeepWorld")
  (Physics|SetSimulatePhysics (Variables|Default|GetCube) true)
  (Input|DisableInput (Game|GetPlayerController 0)))

(fn ConstructionScript)