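; BP_Ethan_Controlled is an AI-driven pawn that moves to a target position through its AI controller.
; On BeginPlay it binds a move event via BindEventToAI, randomizes Cube1's mass override and starts a looping timer that invokes CallAI every few seconds.
; The bound event sends the pawn to TargetPos with navigation projection; BindEventToAI and CallAI are defined outside this graph.
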(event Custom|CustomEvent
  (AI|Navigation|MovetoLocation (AI|GetAIController self) (Variables|Default|GetTargetPos) -1.0 true true true true 0))

(event EventBeginPlay
  (EventDispatchers|BindEventtoAI (delegate Custom|CustomEvent))
  (Utilities|Time|SetTimerbyFunctionName 0 "SetRandomPos" 5.0 true)
  (Class|PrimitiveComponent|SetMassOverrideinKg (Variables|Default|GetCube1) "None" (Math|Random|RandomFloatinRange 3.0 6e+01) true))

(fn ConstructionScript
  (|CallParentFunction))

(fn SetRandomPos
  (Default|CallAI))