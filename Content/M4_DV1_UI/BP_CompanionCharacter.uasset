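; Companion character that follows the local player and carries an indicator widget that faces the camera.
; Each tick, while CompanionState is Following, it issues a SimpleMoveToActor toward player pawn 0 whenever that pawn is beyond FollowDistance, comparing squared distances.
; Every tick, regardless of state, AlignUI billboards IndicatorWidget by rotating it toward the player camera manager's location.
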(event EventBeginPlay)

(event Collision|EventActorBeginOverlap
  (params (OtherActor :type Actor%20Object%20Reference)))

(event EventTick
  (params (DeltaSeconds :type Float%20%28single-precision%29))
  (Utilities|FlowControl|Sequence
    (:then_0
      (switch Utilities|FlowControl|Switch|SwitchonECompanionState (Variables|Default|GetCompanionState)
        (:NewEnumerator0
          (CallFunction|FollowPlayer))))
    (:then_1
      (UI|AlignUI))))

(fn ConstructionScript
  (|CallParentFunction))

(fn FollowPlayer
  (bind _output_get (LocalVariables|SetLocalPlayerPawn (Game|Player|GetPlayerPawn 0)))
  (if (> (Transformation|GetSquaredDistanceTo _output_get self) (Math|Float|Square (Variables|Default|GetFollowDistance)))
    (AI|Navigation|SimpleMovetoActor (Pawn|GetController) (LocalVariables|GetLocalPlayerPawn))
    (return)
    (else
      (return))))

(fn AlignUI
  (bind _indicator_widget (Variables|Default|GetIndicator%20Widget))
  (Transformation|SetWorldRotation _indicator_widget (Math|Rotator|FindLookatRotation (Transformation|GetWorldLocation _indicator_widget) (Transformation|GetActorLocation (Game|GetPlayerCameraManager 0))) false false)
  (return))