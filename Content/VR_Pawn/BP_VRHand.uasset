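; VR hand actor that follows a left or right motion controller and grabs and drops objects implementing BPI_PickupActor.
; While empty-handed, it searches each tick for the nearest pickup within GrabRadius.
; GrabActor attempts pickup only if that candidate matches the capsule's colliding actor, passing the MotionController through the interface; ReleaseActor sends the drop message.
; Grip axis input drives the hand AnimBP, and the left hand reuses a Z-mirrored mesh.
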(event OnComponentBeginOverlap(Capsule)
  (params (OverlappedComponent :type Primitive%20Component%20Object%20Reference) (OtherActor :type Actor%20Object%20Reference) (OtherComp :type Primitive%20Component%20Object%20Reference) (OtherBodyIndex :type Integer) (bFromSweep :type Boolean) (SweepResult :type Hit%20Result%20Structure%20%28by%20ref%29))
  (Variables|Default|SetbIsColliding true)
  (Variables|Default|SetCollidingActor OtherActor))

(event OnComponentEndOverlap(Capsule)
  (params (OverlappedComponent :type Primitive%20Component%20Object%20Reference) (OtherActor :type Actor%20Object%20Reference) (OtherComp :type Primitive%20Component%20Object%20Reference) (OtherBodyIndex :type Integer))
  (Variables|Default|SetbIsColliding false))

(event EventTick
  (params (DeltaSeconds :type Float%20%28single-precision%29))
  (Utilities|FlowControl|Sequence
    (:then_0
      (Variables|Default|GetHeldActor
        (:then)
        (:else
          (CallFunction|FindNearestPickupObject))))
    (:then_1
      (bind _asabp_mannequin_hand_right (Utilities|Casting|CastToABP_MannequinHand_Right (Components|SkeletalMesh|GetAnimInstance (Variables|Default|GetHandMesh))))
      (Variables|/Game/VR_Pawn/ABP_MannequinHand_Right.ABP_MannequinHand_Right_C|SetGrip _asabp_mannequin_hand_right (select (Utilities|Enum|Equal(Enum) (Variables|Default|GetHand) "Left") (Input|AxisValues|GetGrip_L_Axis) (Input|AxisValues|GetGrip_R_Axis))))))

(fn ConstructionScript
  (bind _hand (Variables|Default|GetHand))
  (Variables|/Script/HeadMountedDisplay.MotionControllerComponent|SetMotionSource (Variables|Default|GetMotionController) (Utilities|Name|EnumtoName _hand))
  (if (Utilities|Enum|Equal(Enum) _hand "Left")
    (Transformation|SetWorldScale3D (Variables|Default|GetHandMesh) "1.000000,1.000000,-1.000000")))

(fn GrabActor
  (Variables|Default|SetbWantsToGrip true)
  (if (Variables|Default|GetbIsColliding)
    (Development|PrintString "Try Grab")
    (Variables|Default|GetHeldActor
      (:then)
      (:else
        (bind _availablepickupactor (Variables|Default|GetAvailablePickupActor)
          (:then
            (if (== _availablepickupactor (Variables|Default|GetCollidingActor))
              (Class|BPIPickupActor|Pickup(Message) _availablepickupactor (Variables|Default|GetMotionController))
              (Variables|Default|SetHeldActor _availablepickupactor)
              (return)
              (else
                (Development|PrintString "Avail wasn't colliding"))))
          (:else
            (Development|PrintString "Available wasn't valid")))))))

(fn ReleaseActor
  (Variables|Default|SetbWantsToGrip false)
  (bind _heldactor (Variables|Default|GetHeldActor)
    (:then
      (if true
        (Class|BPIPickupActor|Drop(Message) _heldactor))
      (Variables|Default|SetHeldActor 0)
      (return))
    (:else
      (return))))

(fn FindNearestPickupObject
  (bind _outactors (Actor|GetAllActorswithInterface "/Game/VR_Pawn/BPI_PickupActor.BPI_PickupActor_C"))
  (for _array_element _outactors
    (bind _output_get (LocalVariables|SetLCL_Curr_Actor_DistSqr (Math|Vector|VectorLengthSquared (- (Transformation|GetActorLocation _array_element) (Transformation|GetWorldLocation (Variables|Default|GetHandMesh))))))
    (if (<= _output_get (Math|Float|Square (Variables|Default|GetGrabRadius)))
      (if (< (LocalVariables|GetLCL_Curr_Actor_DistSqr) (LocalVariables|GetClosest_Range))
        (LocalVariables|SetClosest_Range (LocalVariables|GetLCL_Curr_Actor_DistSqr))
        (LocalVariables|SetNearestPickupActor _array_element))))
  (Variables|Default|SetAvailablePickupActor (LocalVariables|GetNearestPickupActor)))