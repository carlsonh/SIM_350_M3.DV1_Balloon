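; Actor that shows random strings as floating, fading text around itself using three text render components.
; BeginPlay gives each component a dynamic material instance, stored in a map, and starts three staggered looping timers.
; Each update event picks a random string and offset for its text, then a timeline drives vertical drift and material opacity, resetting relative location when finished.
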(event EventBeginPlay
  (bind _output_get (Variables|Default|SetTexts (Utilities|Array|MakeArray (Variables|Default|GetTextRender) (Variables|Default|GetTextRender1) (Variables|Default|GetTextRender2))))
  (for _array_element _output_get
    (bind _returnvalue (Rendering|Material|CreateDynamicMaterialInstance _array_element 0 "/Game/MC/Robotod.Robotod" "None" :!class /Script/Engine.PrimitiveComponent))
    (Utilities|Map|Add (Variables|Default|GetText_DMI_Mat_Map) _array_element _returnvalue))
  (Utilities|Time|SetTimerbyEvent (EventDispatchers|CreateEvent :!event Custom|Update%20Text%201) 8.0 true 2.0)
  (Utilities|Time|SetTimerbyEvent (EventDispatchers|CreateEvent :!event Custom|Update%20Text%202) 8.0 true 4.0)
  (Utilities|Time|SetTimerbyEvent (EventDispatchers|CreateEvent :!event Custom|Update%20Text%203) 8.0 true 7.0))

(event Custom|Update%20Text%201
  (bind _texts (Variables|Default|GetTexts))
  (bind _output (Utilities|Array|Get(acopy) _texts))
  (bind (_text_ _dmi_) (CallFunction|InitializeText _output (.Value (Utilities|Map|Find (Variables|Default|GetText_DMI_Mat_Map) _output))))
  (bind (_direction _text_z _text_opacity) (Timeline|Timeline_0 PlayFromStart)
    (:Update
      (Transformation|AddLocalOffset _text_ (Math|Vector|MakeVector 0.0 0.0 _text_z) false false)
      (Rendering|Material|SetScalarParameterValue _dmi_ "Opacity" _text_opacity :!class /Script/Engine.MaterialInstanceDynamic))
    (:Finished
      (Transformation|SetRelativeLocation _text_ "0, 0, 0" false false))))

(event Custom|Update%20Text%202
  (bind _texts (Variables|Default|GetTexts))
  (bind _output (Utilities|Array|Get(acopy) _texts 1))
  (bind (_text_ _dmi_) (CallFunction|InitializeText _output (.Value (Utilities|Map|Find (Variables|Default|GetText_DMI_Mat_Map) _output))))
  (bind (_direction _text_z _text_opacity) (Timeline|Timeline_1 PlayFromStart)
    (:Update
      (Transformation|AddLocalOffset _text_ (Math|Vector|MakeVector 0.0 0.0 _text_z) false false)
      (Rendering|Material|SetScalarParameterValue _dmi_ "Opacity" _text_opacity :!class /Script/Engine.MaterialInstanceDynamic))
    (:Finished
      (Transformation|SetRelativeLocation _text_ "0, 0, 0" false false))))

(event Custom|Update%20Text%203
  (bind _texts (Variables|Default|GetTexts))
  (bind _output (Utilities|Array|Get(acopy) _texts 2))
  (bind (_text_ _dmi_) (CallFunction|InitializeText _output (.Value (Utilities|Map|Find (Variables|Default|GetText_DMI_Mat_Map) _output))))
  (bind (_direction _text_z _text_opacity) (Timeline|Timeline_2 PlayFromStart)
    (:Update
      (Transformation|AddLocalOffset _text_ (Math|Vector|MakeVector 0.0 0.0 _text_z) false false)
      (Rendering|Material|SetScalarParameterValue _dmi_ "Opacity" _text_opacity :!class /Script/Engine.MaterialInstanceDynamic))
    (:Finished
      (Transformation|SetRelativeLocation _text_ "0, 0, 0" false false))))

(fn ConstructionScript)

(fn InitializeText
  (params (Text :type Text%20Render%20Component%20Object%20Reference) (DMI :type Material%20Instance%20Dynamic%20Object%20Reference))
  (bind _returnvalue (Math|Random|RandomUnitVector))
  (bind _random_strings (Variables|Default|GetRandom%20Strings))
  (bind _random_text_distance (Variables|Default|GetRandom%20Text%20Distance))
  (bind _returnvalue_2 (* _returnvalue _random_text_distance))
  (bind (_x _y _z) (Math|Vector|BreakVector _returnvalue_2))
  (Transformation|AddLocalOffset Text (Math|Vector|MakeVector _x _y (Math|Float|MapRangeClamped _z (- 0.0 _random_text_distance) _random_text_distance -1.5e+02 5e+01)) false false)
  (Rendering|Components|TextRender|SetText Text (Utilities|Text|ToText(String) (Utilities|Array|Get(acopy) _random_strings (Math|Random|RandomInteger (Utilities|Array|Length _random_strings)))))
  (return Text DMI))